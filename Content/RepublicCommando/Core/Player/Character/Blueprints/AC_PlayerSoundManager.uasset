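; AC_PlayerSoundManager is the player's sound component in Republic Commando, playing 2D audio for squad orders and health changes.
; Events cover form up, defend, attack, move to higher ground, health regeneration, health restored and damage taken.
; Each event uses its own DoOnce that resets after a short delay, acting as a per-sound cooldown against overlapping repeats.
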(event `FormUp`
  (`/Engine/EditorBlueprintResources/StandardMacros.DoOnce` false :!label _label
    (:`Completed`
      (`GameplayStatics.PlaySound2D` "/Game/RepublicCommando/Sound/Player/Commands/FormUp/SC_Player_FormUp.SC_Player_FormUp" 1.0 1.0 0.0 null null)
      (`KismetSystemLibrary.Delay` 2.0)
      (goto _label :!via `Reset`))))

(event `DefendPosition`
  (`/Engine/EditorBlueprintResources/StandardMacros.DoOnce` false :!label _label_2
    (:`Completed`
      (`GameplayStatics.PlaySound2D` "/Game/RepublicCommando/Sound/Player/Commands/Defend/SC_Player_Defend.SC_Player_Defend" 1.0 1.0 0.0 null null)
      (`KismetSystemLibrary.Delay` 2.0)
      (goto _label_2 :!via `Reset`))))

(event `OnAttackTarget`
  (`/Engine/EditorBlueprintResources/StandardMacros.DoOnce` false :!label _label_3
    (:`Completed`
      (`GameplayStatics.PlaySound2D` "/Game/RepublicCommando/Sound/Player/Commands/Attack/SC_Player_Attack.SC_Player_Attack" 1.0 1.0 0.0 null null)
      (`KismetSystemLibrary.Delay` 2.0)
      (goto _label_3 :!via `Reset`))))

(event `HealthRestoring`
  (`/Engine/EditorBlueprintResources/StandardMacros.DoOnce` false :!label _label_4
    (:`Completed`
      (`GameplayStatics.PlaySound2D` "/Game/RepublicCommando/Sound/Player/UI/Health/SC_Player_HealthRegen.SC_Player_HealthRegen" 1.0 1.0 0.0 null null)
      (`KismetSystemLibrary.Delay` 0.28)
      (goto _label_4 :!via `Reset`))))

(event `OnHealthRestored`
  (`/Engine/EditorBlueprintResources/StandardMacros.DoOnce` false :!label _label_5
    (:`Completed`
      (`GameplayStatics.PlaySound2D` "/Game/RepublicCommando/Sound/Player/UI/Health/SW_HealthRestored.SW_HealthRestored" 1.0 1.0 0.0 null null)
      (`KismetSystemLibrary.Delay` 5.0)
      (goto _label_5 :!via `Reset`))))

(event `OnHealthDamageReceived`
  (`/Engine/EditorBlueprintResources/StandardMacros.DoOnce` false :!label _label_6
    (:`Completed`
      (`GameplayStatics.PlaySound2D` "/Game/RepublicCommando/Sound/Player/TakeDamage/SC_Player_TakeDamage.SC_Player_TakeDamage" 1.0 1.0 0.0 null null)
      (`KismetSystemLibrary.Delay` 1.5)
      (goto _label_6 :!via `Reset`))))

(event `OnMoveToHigherGround`
  (`/Engine/EditorBlueprintResources/StandardMacros.DoOnce` false :!label _label_7
    (:`Completed`
      (`GameplayStatics.PlaySound2D` "/Game/RepublicCommando/Sound/Player/Special/D38_MoveToHigherGround.D38_MoveToHigherGround" 1.0 1.0 0.0 null null)
      (`KismetSystemLibrary.Delay` 1.5)
      (goto _label_7 :!via `Reset`))))