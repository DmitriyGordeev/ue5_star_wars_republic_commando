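; Plane actor among the player weapon materials that displays a current-versus-maximum amount through material scalar parameters.
; The construction script pushes MaxAmount and CurrentAmount to both Plane0 and Plane1.
; At runtime, OnAmountChange stores the new amount and updates only Plane0.
; BeginPlay also overrides the amount with a hardcoded value after a short delay, again only on Plane0.
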(event `self.ReceiveBeginPlay`
  (`KismetSystemLibrary.Delay` 2.0)
  (set `self.Amount` 2)
  (`MeshComponent.SetScalarParameterValueOnMaterials` (`self.plane_0`) "CurrentAmount" (`KismetMathLibrary.Conv_IntToDouble` (`self.Amount`))))

(event `OnAmountChange`
  (params (NewAmount :type Integer))
  (bind _output_get (set `self.Amount` NewAmount))
  (`MeshComponent.SetScalarParameterValueOnMaterials` (`self.plane_0`) "CurrentAmount" (`KismetMathLibrary.Conv_IntToDouble` _output_get)))

(fn `UserConstructionScript`
  (bind _plane_0 (`self.plane_0`))
  (`MeshComponent.SetScalarParameterValueOnMaterials` _plane_0 "MaxAmount" (`KismetMathLibrary.Conv_IntToDouble` (`self.MaxAmount`)))
  (`MeshComponent.SetScalarParameterValueOnMaterials` _plane_0 "CurrentAmount" (`KismetMathLibrary.Conv_IntToDouble` (`self.Amount`)))
  (`MeshComponent.SetScalarParameterValueOnMaterials` (`self.plane_1`) "MaxAmount" (`KismetMathLibrary.Conv_IntToDouble` (`self.MaxAmount`)))
  (`MeshComponent.SetScalarParameterValueOnMaterials` (`self.plane_1`) "CurrentAmount" (`KismetMathLibrary.Conv_IntToDouble` (`self.Amount`))))