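; Player rifle Blueprint that tracks magazine and total ammo and supplies the muzzle socket location for shooting.
; ConsumeMag decrements both counts and reports success, while Reload refills the magazine without checking or changing the total.
; Magazine count drives material parameters on the Mag mesh as an ammo readout, and total ammo updates a WBP_Ammo widget component.
; Construction sets the magazine capacity, fills it and disables collision on both meshes.
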(event `self.ReceiveBeginPlay`
  (`self.SetAmmoTotal` (`self.TotalAmmo`)))

(fn `ConsumeMag`
  (returns (Success :type Boolean))
  ;[1 1 1] Consumes (shoots) 1 ammo
  (if (> (`self.AmmoMag`) 0)
    (`self.SetAmmoMag` (- (`self.AmmoMag`) 1))
    (`self.SetAmmoTotal` (- (`self.TotalAmmo`) 1))
    (return true)
    (else
      (return false))))

(fn `GetMuzzleLoc`
  (returns (Location :type "Vector Structure"))
  (return (`SceneComponent.GetSocketLocation` (`self.Rifle`) "muzzle")))

(fn `Reload`
  (`self.SetAmmoMag` (`self.MaxAmount`)))

(fn `SetAmmoMag`
  (params (NewValue :type Integer))
  (set `self.AmmoMag` NewValue)
  (`MeshComponent.SetScalarParameterValueOnMaterials` (`self.Mag`) "CurrentAmount" (`KismetMathLibrary.Conv_IntToDouble` (`self.AmmoMag`))))

(fn `SetAmmoTotal`
  (params (NewValue :type Integer))
  (bind _output_get (set `self.TotalAmmo` NewValue))
  (bind _aswbp_ammo (cast `/Game/RepublicCommando/Core/Player/RifleAnim/WBP_Ammo` (`WidgetComponent.GetUserWidgetObject` (`self.AmmoWidget`))))
  (set `TextBlock.Text` (`KismetTextLibrary.Conv_IntToText` _output_get) (`/Game/RepublicCommando/Core/Player/RifleAnim/WBP_Ammo.TB_Ammo` _aswbp_ammo)))

(fn `UserConstructionScript`
  (`MeshComponent.SetScalarParameterValueOnMaterials` (`self.Mag`) "MaxAmount" (`KismetMathLibrary.Conv_IntToDouble` (`self.MaxAmount`)))
  (`self.Reload`)
  (`PrimitiveComponent.SetCollisionEnabled` (`self.Rifle`) "NoCollision")
  (`PrimitiveComponent.SetCollisionEnabled` (`self.Mag`) "NoCollision"))