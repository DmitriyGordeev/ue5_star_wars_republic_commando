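; Projectile fired by clone units that damages what it hits through the IBP_Damagable interface and reports shot accuracy to the shooter.
; On sphere hit it ignores other projectiles, otherwise it prints the instigator's name, counts the hit, applies CarriedDamage and destroys itself.
; A C_Clone instigator's HitCount rises on TargetEnemy hits; other hits trigger OnMaxFailedHits once sequence number minus HitCount reaches MaxFailedHitCount.
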(event `self.Sphere.OnComponentHit`
  (params (HitComponent :type "PrimitiveComponent Object Reference") (OtherActor :type "Actor Object Reference") (OtherComp :type "PrimitiveComponent Object Reference") (NormalImpulse :type "Vector Structure") (Hit :type "HitResult Structure (by ref)"))
  (bind (_hitinstigator _hitotherprojectile) (`self.HitResponse` Hit))
  (if _hitotherprojectile
    (`PrimitiveComponent.IgnoreActorWhenMoving` (`self.Sphere`) OtherActor true)
    (else
      (`KismetSystemLibrary.PrintString` (`KismetSystemLibrary.GetDisplayName` (`self.Instigator`)))
      (if true
        (`self.CountHits` OtherActor)
        (message `/Game/RepublicCommando/Core/Interfaces/IBP_Damagable.ConsumeDamage` OtherActor (`self.CarriedDamage`)) ; If actor is IBP_Damagable - call ConsumeDamage( . ) otherwise ignore
        (`self.K2_DestroyActor`)))))

(fn `CountHits`
  (params (HitActor :type "Actor Object Reference"))
  (bind _asc_clone (cast `/Game/RepublicCommando/Characters/Clone/C_Clone` (`self.GetInstigator`)))
  (if (== (`BaseNPCCharacter.TargetEnemy` _asc_clone) HitActor)
    (`/Engine/EditorBlueprintResources/StandardMacros.IncrementInt` (`/Game/RepublicCommando/Characters/Clone/C_Clone.HitCount` _asc_clone))
    (else
      (`self.NotifyMaxFailedHits` _asc_clone))))

(fn `NotifyMaxFailedHits`
  (params (Clone :type "/Game/RepublicCommando/Characters/Clone/C_Clone Object Reference"))
  (if (>= (- (`self.NumInShootingSequence`) (`/Game/RepublicCommando/Characters/Clone/C_Clone.HitCount` Clone)) (`/Game/RepublicCommando/Characters/Clone/C_Clone.MaxFailedHitCount` Clone))
    (`/Game/RepublicCommando/Characters/Clone/C_Clone.OnMaxFailedHits` Clone)))

(fn `UserConstructionScript`
  (`parent.UserConstructionScript`))