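; BP_Droid_RocketProjectile is a droid rocket projectile that builds on a parent projectile class.
; Before damage is applied, it spawns the rocket explosion Niagara system and plays a barrel sound at its own location.
; SetVFXDirection stores the given direction and passes it to the blaster ribbon Niagara component as its direction parameter.
; BeginPlay and the construction script only call their parent versions.
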(event `self.ReceiveBeginPlay`
  (`parent.ReceiveBeginPlay`))

(event `self.OnBeforeDamage`
  (params (Hit :type "HitResult Structure"))
  (bind _returnvalue (`self.K2_GetActorLocation`))
  (`NiagaraFunctionLibrary.SpawnSystemAtLocation` "/Game/RepublicCommando/VFX/DroidRocket/RocketExplosionAtHit/NS_RocketExplosion.NS_RocketExplosion" _returnvalue)
  (`GameplayStatics.PlaySoundAtLocation` "/Game/RepublicCommando/Sound/SuperBattleDroid/Explosion/SW_barrel_02.SW_barrel_02" _returnvalue (struct) 1.0 1.0 0.0 null null null null))

(fn `SetVFXDirection`
  (params (Direction :type "Vector Structure"))
  (bind _output_get (set `self.VFXDirection` Direction))
  (`FXSystemComponent.SetVectorParameter` (`self.NiagaraBlasterRibbon`) "u_direction" _output_get))

(fn `UserConstructionScript`
  (`parent.UserConstructionScript`))