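; Projectile that applies its carried damage to droids and reports shooting accuracy to the clone that fired it.
; On sphere hit, it raises the clone's hit count for the target enemy or checks for excess misses otherwise, then damages any droid and destroys itself.
; A still-live projectile repeats the miss check after a delay, where a noted bug risk is reading an already reset hit count.
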(event `self.ReceiveBeginPlay`
  (`KismetSystemLibrary.Delay` 10.0)
  (`/Engine/EditorBlueprintResources/StandardMacros.IsValid` self
    (:`Is Valid`
      (bind _asc_clone (cast `/Game/RepublicCommando/Characters/Clone/C_Clone` (`self.Instigator`)))
      ;[1 0.7019 0.7019] May produce a bug when clone finished shooting sequence, and at the ned HitCounter reset to 0, but NotifyMaxFailedHits( ) will still use it (refreshed and not relevant value) for calculating Failed hits
      (`self.NotifyMaxFailedHits` _asc_clone))))

(event `self.Sphere.OnComponentHit`
  (params (HitComponent :type "PrimitiveComponent Object Reference") (OtherActor :type "Actor Object Reference") (OtherComp :type "PrimitiveComponent Object Reference") (NormalImpulse :type "Vector Structure") (Hit :type "HitResult Structure (by ref)"))
  (`|ExecutionSequence`
    (:`then_0`
      (`self.CloneHitCounter` OtherActor))
    (:`then_1`
      (bind _asc_droid (cast `/Game/RepublicCommando/Characters/Droid/C_Droid` OtherActor))
      (`/Game/RepublicCommando/Characters/Droid/C_Droid.ConsumeDamage` _asc_droid (`self.CarriedDamage`)))
    (:`then_2`
      (`self.K2_DestroyActor`))))

(fn `CloneHitCounter`
  (params (HitActor :type "Actor Object Reference"))
  (bind _asc_clone (cast `/Game/RepublicCommando/Characters/Clone/C_Clone` (`self.GetInstigator`)))
  (if (== HitActor (`BaseNPCCharacter.TargetEnemy` _asc_clone))
    (`/Engine/EditorBlueprintResources/StandardMacros.IncrementInt` (`/Game/RepublicCommando/Characters/Clone/C_Clone.HitCount` _asc_clone))
    (else
      (`self.NotifyMaxFailedHits` _asc_clone))))

(fn `NotifyMaxFailedHits`
  (params (Clone :type "/Game/RepublicCommando/Characters/Clone/C_Clone Object Reference"))
  (if (>= (- (`self.NumInShootingSequence`) (`/Game/RepublicCommando/Characters/Clone/C_Clone.HitCount` Clone)) (`/Game/RepublicCommando/Characters/Clone/C_Clone.MaxFailedHitCount` Clone))
    (`/Game/RepublicCommando/Characters/Clone/C_Clone.OnMaxFailedHits` Clone)))

(fn `UserConstructionScript`)