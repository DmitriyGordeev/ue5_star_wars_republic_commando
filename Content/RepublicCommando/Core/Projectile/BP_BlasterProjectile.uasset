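; Blaster projectile actor with a Sphere collision component, which destroys itself after a fixed lifetime if nothing stops it.
; Sphere hits pass to HitResponse, which ignores the instigator and projectiles of the same class.
; Any other hit stops physics, destroys the projectile and spawns a Niagara spark burst and BP_BlasterHitDecal, both oriented by the impact normal.
; The Blueprint's graphs apply no damage.
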(event `self.ReceiveBeginPlay`
  (`KismetSystemLibrary.Delay` 10.0)
  (`self.K2_DestroyActor`))

(event `self.Sphere.OnComponentHit`
  (params (HitComponent :type "PrimitiveComponent Object Reference") (OtherActor :type "Actor Object Reference") (OtherComp :type "PrimitiveComponent Object Reference") (NormalImpulse :type "Vector Structure") (Hit :type "HitResult Structure (by ref)"))
  (`self.HitResponse` Hit))

(fn `HitResponse`
  (params (Hit :type "HitResult Structure"))
  (returns (HitInstigator :type Boolean) (HitOtherProjectile :type Boolean))
  (bind (_bblockinghit _binitialoverlap _time _distance _location _impactpoint _normal _impactnormal _physmat _hitactor) (`GameplayStatics.BreakHitResult` Hit))
  (if (== (`self.Instigator`) _hitactor)
    (return true false)
    (elif (== (`GameplayStatics.GetObjectClass` _hitactor) (`GameplayStatics.GetObjectClass` self))
      (return false true)
      (else
        (`self.PlayHitVFX` Hit)
        (return false false)))))

(fn `PlayHitVFX`
  (params (HitResult :type "HitResult Structure"))
  (bind (_bblockinghit _binitialoverlap _time _distance _location _impactpoint _normal) (`GameplayStatics.BreakHitResult` HitResult))
  (`PrimitiveComponent.SetSimulatePhysics` (`self.Sphere`) false)
  (`self.K2_DestroyActor`)
  (bind _returnvalue (`NiagaraFunctionLibrary.SpawnSystemAtLocation` "/Game/RepublicCommando/VFX/Blaster/NS_SparksExplosion.NS_SparksExplosion" (+ _impactpoint (* _normal 10.0))))
  (`NiagaraComponent.SetVariableVec3` _returnvalue "Axis" _normal)
  (`|SpawnActorFromClass` "/Game/RepublicCommando/Core/Projectile/BP_BlasterHitDecal.BP_BlasterHitDecal_C" (`KismetMathLibrary.MakeTransform` _impactpoint (`KismetMathLibrary.Quat_Rotator` (`KismetMathLibrary.Conv_VectorToQuaternion` _normal))) "AlwaysSpawn" "OverrideRootScale" null 5.0 5.0 null))

(fn `UserConstructionScript`)